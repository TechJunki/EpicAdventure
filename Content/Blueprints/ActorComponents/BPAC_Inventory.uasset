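; Inventory actor component that stores items picked up by the boy or girl player character.
; AddItem appends the item to the inventory array and prints it for debugging.
; It then casts the owner to BP_ATB_BOY, falling back to BP_ATB_GIRL, and passes the item to that character's inventory widget and equipment component.
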(fn `AddItem`
  (params (NewItem :type "String (by ref)"))
  (bind _returnvalue (`self.GetOwner`))
  (`KismetArrayLibrary.Array_Add` (`self.InventoryArray`) NewItem)
  (`KismetSystemLibrary.PrintString` NewItem)
  (bind _asbp_atb_boy (cast `/Game/ArcaneToyboxAssets/Character_Quin/CharacterBlueprint/BP_ATB_BOY` _returnvalue)
    (:`then`
      (`/Game/Blueprints/UI/Inventory.AddItem` (`/Game/ArcaneToyboxAssets/Character_Quin/CharacterBlueprint/BP_ATB_BOY.InventoryWidget` _asbp_atb_boy) NewItem)
      (`/Game/Blueprints/UI/CharacterEquipment.AddCharacterEquipment` (`/Game/ArcaneToyboxAssets/Character_Quin/CharacterBlueprint/BP_ATB_BOY.CharacterEquipment` _asbp_atb_boy) NewItem))
    (:`CastFailed`
      (bind _asbp_atb_girl (cast `/Game/ArcaneToyboxAssets/Character_Abbi/CharacterBlueprint/BP_ATB_GIRL` _returnvalue))
      (`/Game/Blueprints/UI/Inventory.AddItem` (`/Game/ArcaneToyboxAssets/Character_Abbi/CharacterBlueprint/BP_ATB_GIRL.InventoryWidget` _asbp_atb_girl) NewItem)
      (`/Game/Blueprints/UI/CharacterEquipment.AddCharacterEquipment` (`/Game/ArcaneToyboxAssets/Character_Abbi/CharacterBlueprint/BP_ATB_GIRL.CharacterEquipment` _asbp_atb_girl) NewItem))))