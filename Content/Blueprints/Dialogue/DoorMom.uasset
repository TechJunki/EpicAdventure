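; DoorMom is an interactable door that opens the mom's sword dialogue through its ACMomSwordDialogue component.
; Player overlap toggles the door's outline through ACOutlinerAdvanced.
; On entry, a "symbol" tag on the door mesh component also triggers a replicated exclamation-mark spawn and a leftover debug print.
; On exit, any attached symbol is found and destroyed.
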(event `/Game/Blueprints/Dialogue/BPI_Interactable.Interact`
  (params (Instigator :type "Actor Object Reference"))
  (set `self.InteractInstigator` Instigator)
  (`/Game/Blueprints/Dialogue/AC_Dialogue_Base.OpenConversation` (`self.AC_MomSwordDialogue`)))

(event `self.ReceiveActorBeginOverlap`
  (params (OtherActor :type "Actor Object Reference"))
  (if (== OtherActor (`GameplayStatics.GetPlayerCharacter` 0))
    (set `self.Overlapped?` true)
    (`/Game/Hyper/Outliner_System/Blueprints/AC_Outliner_Abstract.Switch Outline On Actor` (`self.AC_Outliner_Advanced`) self "NewEnumerator1" (`self.Overlapped?`) "NewEnumerator2")
    (if (`ActorComponent.ComponentHasTag` (`self.SM_ATB_ModularBuilding_Deco_Door_WindowSquare`) "symbol")
      (`/Game/Hyper/Outliner_System/Blueprints/AC_Outliner_Abstract.Server: Spawn Replicated Symbol` (`self.AC_Outliner_Advanced`) (`KismetMathLibrary.MakeTransform` (-100.0 100.0 150.0) (struct) (3.0 3.0 3.0)) true 15.0 1.0 true 1.0 "/Game/Hyper/ResourcePack/Props/Symbols/Mesh/SM_Symbol_ExclamationMark.SM_Symbol_ExclamationMark" "symbol" true self)
      (`KismetSystemLibrary.PrintString` "SPAWNEDDDD"))))

(event `self.ReceiveActorEndOverlap`
  (params (OtherActor :type "Actor Object Reference"))
  (bind _ac_outliner_advanced (`self.AC_Outliner_Advanced`))
  (bind (_symbol_attached _symbol_actor_attached) (`/Game/Hyper/Outliner_System/Blueprints/AC_Outliner_Abstract.Check if actor has symbol attached` _ac_outliner_advanced self))
  (if (== (`GameplayStatics.GetPlayerCharacter` 0) OtherActor)
    (set `self.Overlapped?` false)
    (`/Game/Hyper/Outliner_System/Blueprints/AC_Outliner_Abstract.Switch Outline On Actor` (`self.AC_Outliner_Advanced`) self "NewEnumerator1" (`self.Overlapped?`) "NewEnumerator2")
    (if _symbol_attached
      (`/Game/Hyper/Outliner_System/Blueprints/AC_Outliner_Abstract.Destroy symbol by actror` _ac_outliner_advanced _symbol_actor_attached))))

(fn `UserConstructionScript`
  (`parent.UserConstructionScript`))