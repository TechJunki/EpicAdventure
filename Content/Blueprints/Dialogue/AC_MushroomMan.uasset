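; Dialogue component for Shrumer, the Mycomancer mushroom NPC who summons the player to Florathia and gives the opening quest.
; Overrides Dialogue and switches on ActiveDialogueBranch: the default intro is a three-way option tree whose paths converge on gathering magical artifacts and set the QuestStart branch.
; QuestStart asks if the player is ready, then either moves to TalkAfterQuestStart with directions to the Forest of Whispers or clears progress.
; TalkAfterQuestStart repeats a short reminder.
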(fn `Dialogue`
  (`parent.Dialogue`)
  (switch `name` (`self.ActiveDialogueBranch`)
    (:`Default`
      (bind (_dialoguestate _optionindex) (`self.AddDialogue` "Shrumer" "Holy. MooMoo. IT ACTUALLY WORKED!!!" (`|MakeArray` (make `/Game/Blueprints/Dialogue/Struct_Options` "What worked?") (make `/Game/Blueprints/Dialogue/Struct_Options` "Where am I?") (make `/Game/Blueprints/Dialogue/Struct_Options` "What are you?") :!type "/Game/Blueprints/Dialogue/Struct_Options Structure")))
      (switch `/Game/Blueprints/Dialogue/Enum_DialogueState` _dialoguestate
        (:`NewEnumerator0`
          (switch `int` _optionindex
            (:`0`
              ;[0 0 0 1 218] MushroomManDefault1
              (bind _dialoguestate_2 (`self.AddDialogue` "Shrumer" "The ancient spell I found!" (`|MakeArray`)))
              (switch `/Game/Blueprints/Dialogue/Enum_DialogueState` _dialoguestate_2
                (:`NewEnumerator0`
                  (bind (_dialoguestate_3 _optionindex_2) (`self.AddDialogue` "Shrumer" "It's said that this spell will travel the realms until it finds the one true hero who can bring balance back to the land." (`|MakeArray` (make `/Game/Blueprints/Dialogue/Struct_Options` "Balance? What kind of balance?") (make `/Game/Blueprints/Dialogue/Struct_Options` "A hero? I’m just a kid!") (make `/Game/Blueprints/Dialogue/Struct_Options` "Tell me more about this spell.") :!type "/Game/Blueprints/Dialogue/Struct_Options Structure")))
                  (switch `/Game/Blueprints/Dialogue/Enum_DialogueState` _dialoguestate_3
                    (:`NewEnumerator0`
                      (switch `int` _optionindex_2
                        (:`0`
                          (bind (_dialoguestate_4 _optionindex_3) (`self.AddDialogue` "Shrumer" "Our land is in chaos! The elements are out of whack, the seasons are all mixed up, and our creatures are confused. We need someone brave and clever to set things right." (`|MakeArray` (make `/Game/Blueprints/Dialogue/Struct_Options` "That sounds serious. How can I help?") (make `/Game/Blueprints/Dialogue/Struct_Options` "Is there a reward for this?") (make `/Game/Blueprints/Dialogue/Struct_Options` "Can I go back home after this?") :!type "/Game/Blueprints/Dialogue/Struct_Options Structure")))
                          (switch `/Game/Blueprints/Dialogue/Enum_DialogueState` _dialoguestate_4
                            (:`NewEnumerator0`
                              (switch `int` _optionindex_3
                                (:`0`
                                  _)
                                (:`1`
                                  (bind (_dialoguestate_5 _optionindex_4) (`self.AddDialogue` "Shrumer" "Of course! You’ll be celebrated as the greatest hero in our land. Plus, you’ll get to keep any treasures you find along the way!" (`|MakeArray` (make `/Game/Blueprints/Dialogue/Struct_Options` "Okay! How can I help?") :!type "/Game/Blueprints/Dialogue/Struct_Options Structure")))
                                  (switch `/Game/Blueprints/Dialogue/Enum_DialogueState` _dialoguestate_5
                                    (:`NewEnumerator0`
                                      (switch `int` _optionindex_4
                                        (:`0`
                                          _)))))
                                (:`2`
                                  (bind (_dialoguestate_6 _optionindex_5) (`self.AddDialogue` "Shrumer" "Yes, once the balance is restored, the portal will open again, and you can return home whenever you wish." (`|MakeArray` (make `/Game/Blueprints/Dialogue/Struct_Options` "I better hurry then so mom isn't worried I am gone!") :!type "/Game/Blueprints/Dialogue/Struct_Options Structure")))
                                  (switch `/Game/Blueprints/Dialogue/Enum_DialogueState` _dialoguestate_6
                                    (:`NewEnumerator0`
                                      (switch `int` _optionindex_5
                                        (:`0`
                                          _))))))
                              (bind _dialoguestate_7 (`self.AddDialogue` "Shrumer" "Your bravery is inspiring! First, you'll need to gather some magical artifacts. They are hidden in different parts of our realm." (`|MakeArray`)))
                              (switch `/Game/Blueprints/Dialogue/Enum_DialogueState` _dialoguestate_7
                                (:`NewEnumerator0`
                                  (`self.SetDialogueBranch` "QuestStart")
                                  (`self.CloseConversation`))))))
                        (:`1`
                          (bind (_dialoguestate_8 _optionindex_6) (`self.AddDialogue` "Shrumer" "Ah, but sometimes the greatest heroes come from the most unexpected places. Your heart and spirit are what we need!" (`|MakeArray` (make `/Game/Blueprints/Dialogue/Struct_Options` "If you say so... What’s the first step?") (make `/Game/Blueprints/Dialogue/Struct_Options` "Are you sure there’s no mistake?") (make `/Game/Blueprints/Dialogue/Struct_Options` "What’s in it for me?") :!type "/Game/Blueprints/Dialogue/Struct_Options Structure")))
                          (switch `/Game/Blueprints/Dialogue/Enum_DialogueState` _dialoguestate_8
                            (:`NewEnumerator0`
                              (switch `int` _optionindex_6
                                (:`0`
                                  _)
                                (:`1`
                                  (bind (_dialoguestate_9 _optionindex_7) (`self.AddDialogue` "Shrumer" "Positive! The spell only works on those with true hero potential. I believe in you!" (`|MakeArray` (make `/Game/Blueprints/Dialogue/Struct_Options` "Okay! How can I help?") :!type "/Game/Blueprints/Dialogue/Struct_Options Structure")))
                                  (switch `/Game/Blueprints/Dialogue/Enum_DialogueState` _dialoguestate_9
                                    (:`NewEnumerator0`
                                      (switch `int` _optionindex_7
                                        (:`0`
                                          _)))))
                                (:`2`
                                  (bind (_dialoguestate_10 _optionindex_8) (`self.AddDialogue` "Shrumer" "You’ll be celebrated as the greatest hero in our land and get to keep any treasures you find along the way!" (`|MakeArray` (make `/Game/Blueprints/Dialogue/Struct_Options` "Okay! How can I help?") :!type "/Game/Blueprints/Dialogue/Struct_Options Structure")))
                                  (switch `/Game/Blueprints/Dialogue/Enum_DialogueState` _dialoguestate_10
                                    (:`NewEnumerator0`
                                      (switch `int` _optionindex_8
                                        (:`0`
                                          _))))))
                              (bind _dialoguestate_11 (`self.AddDialogue` "Shrumer" "First, you’ll need to gather some magical artifacts. They are hidden in different parts of our realm" (`|MakeArray`)))
                              (switch `/Game/Blueprints/Dialogue/Enum_DialogueState` _dialoguestate_11
                                (:`NewEnumerator0`
                                  (`self.SetDialogueBranch` "QuestStart")
                                  (`self.CloseConversation`))))))
                        (:`2`
                          (bind (_dialoguestate_12 _optionindex_9) (`self.AddDialogue` "Shrumer" "The spell is ancient magic, passed down through generations. It seeks out the pure of heart, those who can bring balance and harmony." (`|MakeArray` (make `/Game/Blueprints/Dialogue/Struct_Options` "Interesting! So, what do I do now?") (make `/Game/Blueprints/Dialogue/Struct_Options` "Magic, huh? Can I learn any spells?") (make `/Game/Blueprints/Dialogue/Struct_Options` "What happens if I fail?") :!type "/Game/Blueprints/Dialogue/Struct_Options Structure")))
                          (switch `/Game/Blueprints/Dialogue/Enum_DialogueState` _dialoguestate_12
                            (:`NewEnumerator0`
                              (switch `int` _optionindex_9
                                (:`0`
                                  _)
                                (:`1`
                                  (bind (_dialoguestate_13 _optionindex_10) (`self.AddDialogue` "Shrumer" "Absolutely! Along your journey, you’ll discover magical runes that grant you new abilities." (`|MakeArray` (make `/Game/Blueprints/Dialogue/Struct_Options` "Okay! How can I help?") :!type "/Game/Blueprints/Dialogue/Struct_Options Structure")))
                                  (switch `/Game/Blueprints/Dialogue/Enum_DialogueState` _dialoguestate_13
                                    (:`NewEnumerator0`
                                      (switch `int` _optionindex_10
                                        (:`0`
                                          _)))))
                                (:`2`
                                  (bind (_dialoguestate_14 _optionindex_11) (`self.AddDialogue` "Shrumer" "Failure isn’t an option for a true hero! But don’t worry, I’ll be here to guide you through your journey." (`|MakeArray` (make `/Game/Blueprints/Dialogue/Struct_Options` "Okay! How can I help?") :!type "/Game/Blueprints/Dialogue/Struct_Options Structure")))
                                  (switch `/Game/Blueprints/Dialogue/Enum_DialogueState` _dialoguestate_14
                                    (:`NewEnumerator0`
                                      (switch `int` _optionindex_11
                                        (:`0`
                                          _))))))
                              (bind _dialoguestate_15 (`self.AddDialogue` "Shrumer" "First, you’ll need to gather some magical artifacts. They are hidden in different parts of our realm." (`|MakeArray`)))
                              (switch `/Game/Blueprints/Dialogue/Enum_DialogueState` _dialoguestate_15
                                (:`NewEnumerator0`
                                  (`self.SetDialogueBranch` "QuestStart")
                                  (`self.CloseConversation`))))))))))))
            (:`1`
              ;[0 0 0 1 218] MushroomManDefault2
              (bind (_dialoguestate_16 _optionindex_12) (`self.AddDialogue` "Shrumer" "Welcome to the land of Florathia, a place of magic and wonder! But currently, it's a bit of a mess." (`|MakeArray` (make `/Game/Blueprints/Dialogue/Struct_Options` "Why is it a mess?") (make `/Game/Blueprints/Dialogue/Struct_Options` "It looks pretty cool to me!") (make `/Game/Blueprints/Dialogue/Struct_Options` "How do I get back home?") :!type "/Game/Blueprints/Dialogue/Struct_Options Structure")))
              (switch `/Game/Blueprints/Dialogue/Enum_DialogueState` _dialoguestate_16
                (:`NewEnumerator0`
                  (switch `int` _optionindex_12
                    (:`0`
                      (bind (_dialoguestate_17 _optionindex_13) (`self.AddDialogue` "Shrumer" "The balance of nature has been disrupted. Seasons are in chaos, creatures are confused, and we need your help to set things right!" (`|MakeArray` (make `/Game/Blueprints/Dialogue/Struct_Options` "How can I help?") (make `/Game/Blueprints/Dialogue/Struct_Options` "What caused this imbalance?") (make `/Game/Blueprints/Dialogue/Struct_Options` "Do I get a reward for helping?") :!type "/Game/Blueprints/Dialogue/Struct_Options Structure")))
                      (switch `/Game/Blueprints/Dialogue/Enum_DialogueState` _dialoguestate_17
                        (:`NewEnumerator0`
                          (switch `int` _optionindex_13
                            (:`0`
                              _)
                            (:`1`
                              (bind (_dialoguestate_18 _optionindex_14) (`self.AddDialogue` "Shrumer" "A dark force has been tampering with the elements, twisting them for its own gain. We must stop it!" (`|MakeArray` (make `/Game/Blueprints/Dialogue/Struct_Options` "Okay! How can I help?") :!type "/Game/Blueprints/Dialogue/Struct_Options Structure")))
                              (switch `/Game/Blueprints/Dialogue/Enum_DialogueState` _dialoguestate_18
                                (:`NewEnumerator0`
                                  (switch `int` _optionindex_14
                                    (:`0`
                                      _)))))
                            (:`2`
                              (bind (_dialoguestate_19 _optionindex_15) (`self.AddDialogue` "Shrumer" "Absolutely! You’ll be hailed as a hero and can keep any treasures you find." (`|MakeArray` (make `/Game/Blueprints/Dialogue/Struct_Options` "Okay! How can I help?") :!type "/Game/Blueprints/Dialogue/Struct_Options Structure")))
                              (switch `/Game/Blueprints/Dialogue/Enum_DialogueState` _dialoguestate_19
                                (:`NewEnumerator0`
                                  (switch `int` _optionindex_15
                                    (:`0`
                                      _))))))
                          (bind _dialoguestate_20 (`self.AddDialogue` "Shrumer" "You’ll need to gather magical artifacts scattered across our realm. They hold the power to restore balance." (`|MakeArray`)))
                          (switch `/Game/Blueprints/Dialogue/Enum_DialogueState` _dialoguestate_20
                            (:`NewEnumerator0`
                              (`self.SetDialogueBranch` "QuestStart")
                              (`self.CloseConversation`))))))
                    (:`1`
                      (bind (_dialoguestate_21 _optionindex_16) (`self.AddDialogue` "Shrumer" "It has its charms, doesn’t it? But underneath the beauty, there’s chaos that needs to be sorted out." (`|MakeArray` (make `/Game/Blueprints/Dialogue/Struct_Options` "What kind of chaos?") (make `/Game/Blueprints/Dialogue/Struct_Options` "What do you need me to do?") (make `/Game/Blueprints/Dialogue/Struct_Options` "Can I explore first?") :!type "/Game/Blueprints/Dialogue/Struct_Options Structure")))
                      (switch `/Game/Blueprints/Dialogue/Enum_DialogueState` _dialoguestate_21
                        (:`NewEnumerator0`
                          (switch `int` _optionindex_16
                            (:`0`
                              (bind (_dialoguestate_22 _optionindex_17) (`self.AddDialogue` "Shrumer" "The seasons are mixed up, creatures are behaving oddly, and natural disasters are rampant. We need to restore harmony." (`|MakeArray` (make `/Game/Blueprints/Dialogue/Struct_Options` "That sounds serious. How can I help?") :!type "/Game/Blueprints/Dialogue/Struct_Options Structure")))
                              (switch `/Game/Blueprints/Dialogue/Enum_DialogueState` _dialoguestate_22
                                (:`NewEnumerator0`
                                  (switch `int` _optionindex_17
                                    (:`0`
                                      (bind _dialoguestate_23 (`self.AddDialogue` "Shrumer" "You’ll need to gather magical artifacts scattered across our realm. They hold the power to restore balance." (`|MakeArray`)))
                                      (switch `/Game/Blueprints/Dialogue/Enum_DialogueState` _dialoguestate_23
                                        (:`NewEnumerator0`
                                          (`self.SetDialogueBranch` "QuestStart")
                                          (`self.CloseConversation`))))))))
                            (:`1`
                              (bind (_dialoguestate_24 _optionindex_18) (`self.AddDialogue` "Shrumer" "Gather magical artifacts scattered across the land. They have the power to fix everything." (`|MakeArray` (make `/Game/Blueprints/Dialogue/Struct_Options` "Okay! I better get started!") (make `/Game/Blueprints/Dialogue/Struct_Options` "Can I explore first?") :!type "/Game/Blueprints/Dialogue/Struct_Options Structure")))
                              (switch `/Game/Blueprints/Dialogue/Enum_DialogueState` _dialoguestate_24
                                (:`NewEnumerator0`
                                  (switch `int` _optionindex_18
                                    (:`0`
                                      _)
                                    (:`1`
                                      (bind (_dialoguestate_25 _optionindex_19) (`self.AddDialogue` "Shrumer" "Of course! Exploration is key to finding the artifacts. Just keep an eye out for anything unusual." (`|MakeArray` (make `/Game/Blueprints/Dialogue/Struct_Options` "Okay! I'm gonna go look around.") :!type "/Game/Blueprints/Dialogue/Struct_Options Structure") :!label _label))
                                      (switch `/Game/Blueprints/Dialogue/Enum_DialogueState` _dialoguestate_25
                                        (:`NewEnumerator0`
                                          (switch `int` _optionindex_19
                                            (:`0`
                                              _))))))
                                  (`self.SetDialogueBranch` "QuestStart")
                                  (`self.CloseConversation`))))
                            (:`2`
                              (goto _label))))))
                    (:`2`
                      (bind (_dialoguestate_26 _optionindex_20) (`self.AddDialogue` "Shrumer" "Once balance is restored, the portal will open again, allowing you to return home. In the meantime, enjoy the adventure!" (`|MakeArray` (make `/Game/Blueprints/Dialogue/Struct_Options` "Sounds fair. What’s the first step?") (make `/Game/Blueprints/Dialogue/Struct_Options` "How long will this take?") (make `/Game/Blueprints/Dialogue/Struct_Options` "Can you promise I’ll be safe?") :!type "/Game/Blueprints/Dialogue/Struct_Options Structure")))
                      (switch `/Game/Blueprints/Dialogue/Enum_DialogueState` _dialoguestate_26
                        (:`NewEnumerator0`
                          (switch `int` _optionindex_20
                            (:`0`
                              (bind (_dialoguestate_27 _optionindex_21) (`self.AddDialogue` "Shrumer" "Gather magical artifacts scattered across the land. They have the power to fix everything." (`|MakeArray` (make `/Game/Blueprints/Dialogue/Struct_Options` "Okay! I better get started!") (make `/Game/Blueprints/Dialogue/Struct_Options` "Can I explore first?") :!type "/Game/Blueprints/Dialogue/Struct_Options Structure")))
                              (switch `/Game/Blueprints/Dialogue/Enum_DialogueState` _dialoguestate_27
                                (:`NewEnumerator0`
                                  (switch `int` _optionindex_21
                                    (:`0`
                                      _)
                                    (:`1`
                                      (bind (_dialoguestate_28 _optionindex_22) (`self.AddDialogue` "Shrumer" "Of course! Exploration is key to finding the artifacts. Just keep an eye out for anything unusual." (`|MakeArray` (make `/Game/Blueprints/Dialogue/Struct_Options` "Okay! I'm gonna go look around.") :!type "/Game/Blueprints/Dialogue/Struct_Options Structure")))
                                      (switch `/Game/Blueprints/Dialogue/Enum_DialogueState` _dialoguestate_28
                                        (:`NewEnumerator0`
                                          (switch `int` _optionindex_22
                                            (:`0`
                                              _))))))
                                  (`self.SetDialogueBranch` "QuestStart")
                                  (`self.CloseConversation`))))
                            (:`1`
                              (bind (_dialoguestate_29 _optionindex_23) (`self.AddDialogue` "Shrumer" "It depends on your bravery and cunning. But don’t worry, time flows differently here. You’ll be back home before you know it." (`|MakeArray` (make `/Game/Blueprints/Dialogue/Struct_Options` "Okay! I better get started!") :!type "/Game/Blueprints/Dialogue/Struct_Options Structure")))
                              (switch `/Game/Blueprints/Dialogue/Enum_DialogueState` _dialoguestate_29
                                (:`NewEnumerator0`
                                  (switch `int` _optionindex_23
                                    (:`0`
                                      (bind _dialoguestate_30 (`self.AddDialogue` "Shrumer" "As you explore, you’ll need to gather magical artifacts scattered across our realm. They hold the power to restore balance and get you back home. " (`|MakeArray`) :!label _label_2))
                                      (switch `/Game/Blueprints/Dialogue/Enum_DialogueState` _dialoguestate_30
                                        (:`NewEnumerator0`
                                          (`self.SetDialogueBranch` "QuestStart")
                                          (`self.CloseConversation`))))))))
                            (:`2`
                              (bind (_dialoguestate_31 _optionindex_24) (`self.AddDialogue` "Shrumer" "I can’t promise there won’t be dangers, but I’ll be here to guide you. Plus, heroes always find a way!" (`|MakeArray` (make `/Game/Blueprints/Dialogue/Struct_Options` "Okay! How can I help?") :!type "/Game/Blueprints/Dialogue/Struct_Options Structure")))
                              (switch `/Game/Blueprints/Dialogue/Enum_DialogueState` _dialoguestate_31
                                (:`NewEnumerator0`
                                  (switch `int` _optionindex_24
                                    (:`0`
                                      (goto _label_2))))))))))))))
            (:`2`
              ;[0 0 0 1 218] MushroomManDefault3
              (bind (_dialoguestate_32 _optionindex_25) (`self.AddDialogue` "Shrumer" "I’m a Mycomancer, a guardian of this land. We Mycomancers are magical beings who protect the balance of nature." (`|MakeArray` (make `/Game/Blueprints/Dialogue/Struct_Options` "A Mycomancer? That’s cool!") (make `/Game/Blueprints/Dialogue/Struct_Options` "Why did you bring me here?") (make `/Game/Blueprints/Dialogue/Struct_Options` "Do you have powers?") :!type "/Game/Blueprints/Dialogue/Struct_Options Structure")))
              (switch `/Game/Blueprints/Dialogue/Enum_DialogueState` _dialoguestate_32
                (:`NewEnumerator0`
                  (switch `int` _optionindex_25
                    (:`0`
                      (bind (_dialoguestate_33 _optionindex_26) (`self.AddDialogue` "Shrumer" "Thank you! We’ve been around for centuries, maintaining harmony. But now, we need your help." (`|MakeArray` (make `/Game/Blueprints/Dialogue/Struct_Options` "What do you need me to do?") (make `/Game/Blueprints/Dialogue/Struct_Options` "How do you maintain harmony?") (make `/Game/Blueprints/Dialogue/Struct_Options` "Can I become a Mycomancer too?") :!type "/Game/Blueprints/Dialogue/Struct_Options Structure")))
                      (switch `/Game/Blueprints/Dialogue/Enum_DialogueState` _dialoguestate_33
                        (:`NewEnumerator0`
                          (switch `int` _optionindex_26
                            (:`0`
                              _)
                            (:`1`
                              (bind (_dialoguestate_34 _optionindex_27) (`self.AddDialogue` "Shrumer" "We use ancient spells and artifacts to keep nature in balance. But a dark force has disrupted everything." (`|MakeArray` (make `/Game/Blueprints/Dialogue/Struct_Options` "Okay! How can I help?") :!type "/Game/Blueprints/Dialogue/Struct_Options Structure")))
                              (switch `/Game/Blueprints/Dialogue/Enum_DialogueState` _dialoguestate_34
                                (:`NewEnumerator0`
                                  (switch `int` _optionindex_27
                                    (:`0`
                                      _)))))
                            (:`2`
                              (bind (_dialoguestate_35 _optionindex_28) (`self.AddDialogue` "Shrumer" "With enough courage and heart, anything is possible! Along your journey, you might just find a way." (`|MakeArray` (make `/Game/Blueprints/Dialogue/Struct_Options` "Okay! How can I help?") :!type "/Game/Blueprints/Dialogue/Struct_Options Structure")))
                              (switch `/Game/Blueprints/Dialogue/Enum_DialogueState` _dialoguestate_35
                                (:`NewEnumerator0`
                                  (switch `int` _optionindex_28
                                    (:`0`
                                      _))))))
                          (bind _dialoguestate_36 (`self.AddDialogue` "Shrumer" "Gather magical artifacts scattered across the land. They hold the power to restore balance." (`|MakeArray`)))
                          (switch `/Game/Blueprints/Dialogue/Enum_DialogueState` _dialoguestate_36
                            (:`NewEnumerator0`
                              (`self.SetDialogueBranch` "QuestStart")
                              (`self.CloseConversation`))))))
                    (:`1`
                      (bind (_dialoguestate_37 _optionindex_29) (`self.AddDialogue` "Shrumer" "Our realm is in chaos, and only a true hero can restore balance. The ancient spell chose you for your pure heart and brave spirit." (`|MakeArray` (make `/Game/Blueprints/Dialogue/Struct_Options` "How can I help?") (make `/Game/Blueprints/Dialogue/Struct_Options` "Are you sure I’m the right person?") (make `/Game/Blueprints/Dialogue/Struct_Options` "What’s in it for me?") :!type "/Game/Blueprints/Dialogue/Struct_Options Structure")))
                      (switch `/Game/Blueprints/Dialogue/Enum_DialogueState` _dialoguestate_37
                        (:`NewEnumerator0`
                          (switch `int` _optionindex_29
                            (:`0`
                              _)
                            (:`1`
                              (bind (_dialoguestate_38 _optionindex_30) (`self.AddDialogue` "Shrumer" "Absolutely! The spell wouldn’t have worked if you weren’t the true hero we need." (`|MakeArray` (make `/Game/Blueprints/Dialogue/Struct_Options` "Okay! How can I help?") :!type "/Game/Blueprints/Dialogue/Struct_Options Structure")))
                              (switch `/Game/Blueprints/Dialogue/Enum_DialogueState` _dialoguestate_38
                                (:`NewEnumerator0`
                                  (switch `int` _optionindex_30
                                    (:`0`
                                      _)))))
                            (:`2`
                              (bind (_dialoguestate_39 _optionindex_31) (`self.AddDialogue` "Shrumer" "You’ll be celebrated as the greatest hero in our land and can keep any treasures you find along the way!" (`|MakeArray` (make `/Game/Blueprints/Dialogue/Struct_Options` "Okay! How can I help?") :!type "/Game/Blueprints/Dialogue/Struct_Options Structure")))
                              (switch `/Game/Blueprints/Dialogue/Enum_DialogueState` _dialoguestate_39
                                (:`NewEnumerator0`
                                  (switch `int` _optionindex_31
                                    (:`0`
                                      _))))))
                          (bind _dialoguestate_40 (`self.AddDialogue` "Shrumer" "You’ll need to gather magical artifacts scattered across our realm. They have the power to set things right." (`|MakeArray`)))
                          (switch `/Game/Blueprints/Dialogue/Enum_DialogueState` _dialoguestate_40
                            (:`NewEnumerator0`
                              (`self.SetDialogueBranch` "QuestStart")
                              (`self.CloseConversation`))))))
                    (:`2`
                      (bind (_dialoguestate_41 _optionindex_32) (`self.AddDialogue` "Shrumer" "Yes! I can control nature to some extent, but my powers are limited by the current imbalance. That’s why we need your help." (`|MakeArray` (make `/Game/Blueprints/Dialogue/Struct_Options` "Can you teach me some magic?") (make `/Game/Blueprints/Dialogue/Struct_Options` "What kind of imbalance?") (make `/Game/Blueprints/Dialogue/Struct_Options` "What do we need to do?") :!type "/Game/Blueprints/Dialogue/Struct_Options Structure")))
                      (switch `/Game/Blueprints/Dialogue/Enum_DialogueState` _dialoguestate_41
                        (:`NewEnumerator0`
                          (switch `int` _optionindex_32
                            (:`0`
                              (bind (_dialoguestate_42 _optionindex_33) (`self.AddDialogue` "Shrumer" "Certainly! As you progress, you’ll find magical runes that grant you new abilities. I’ll guide you along the way." (`|MakeArray` (make `/Game/Blueprints/Dialogue/Struct_Options` "Okay! I better get started!") :!type "/Game/Blueprints/Dialogue/Struct_Options Structure")))
                              (switch `/Game/Blueprints/Dialogue/Enum_DialogueState` _dialoguestate_42
                                (:`NewEnumerator0`
                                  (switch `int` _optionindex_33
                                    (:`0`
                                      (bind _dialoguestate_43 (`self.AddDialogue` "Shrumer" "You’ll need to gather magical artifacts scattered across our realm. They have the power to set things right." (`|MakeArray`)))
                                      (switch `/Game/Blueprints/Dialogue/Enum_DialogueState` _dialoguestate_43
                                        (:`NewEnumerator0`
                                          (`self.SetDialogueBranch` "QuestStart")
                                          (`self.CloseConversation`))))))))
                            (:`1`
                              (bind (_dialoguestate_44 _optionindex_34) (`self.AddDialogue` "Shrumer" "The seasons are mixed up, creatures are behaving oddly, and natural disasters are rampant. We must restore harmony." (`|MakeArray` (make `/Game/Blueprints/Dialogue/Struct_Options` "That sounds serious. How can I help?") :!type "/Game/Blueprints/Dialogue/Struct_Options Structure")))
                              (switch `/Game/Blueprints/Dialogue/Enum_DialogueState` _dialoguestate_44
                                (:`NewEnumerator0`
                                  (switch `int` _optionindex_34
                                    (:`0`
                                      (bind _dialoguestate_45 (`self.AddDialogue` "Shrumer" "As you explore, you’ll need to gather magical artifacts scattered across our realm. They hold the power to restore balance and get you back home. " (`|MakeArray`) :!label _label_3))
                                      (switch `/Game/Blueprints/Dialogue/Enum_DialogueState` _dialoguestate_45
                                        (:`NewEnumerator0`
                                          (`self.SetDialogueBranch` "QuestStart")
                                          (`self.CloseConversation`))))))))
                            (:`2`
                              (goto _label_3))))))))))))))
    (:`QuestStart`
      (bind (_dialoguestate_46 _optionindex_35) (`self.AddDialogue` "Shrumer" "Are you ready to get to it!?" (`|MakeArray` (make `/Game/Blueprints/Dialogue/Struct_Options` "Yes! What's first?") (make `/Game/Blueprints/Dialogue/Struct_Options` "Not quite. Still looking around. ") :!type "/Game/Blueprints/Dialogue/Struct_Options Structure")))
      (switch `/Game/Blueprints/Dialogue/Enum_DialogueState` _dialoguestate_46
        (:`NewEnumerator0`
          (switch `int` _optionindex_35
            (:`0`
              (bind _dialoguestate_47 (`self.AddDialogue` "Shrumer" "To start, you’ll need to visit the Forest of Whispers through that entry over there. You'll learn more about the journey ahead when you speak to those who live in the forest. " (`|MakeArray`)))
              (switch `/Game/Blueprints/Dialogue/Enum_DialogueState` _dialoguestate_47
                (:`NewEnumerator0`
                  (`self.SetDialogueBranch` "TalkAfterQuestStart")
                  (`self.CloseConversation`))))
            (:`1`
              (bind _dialoguestate_48 (`self.AddDialogue` "Shrumer" "Okay. Come talk to me again when you're ready to get started." (`|MakeArray`)))
              (switch `/Game/Blueprints/Dialogue/Enum_DialogueState` _dialoguestate_48
                (:`NewEnumerator0`
                  (`self.ClearDialogueProgress`)
                  (`self.CloseConversation`))))))))
    (:`TalkAfterQuestStart`
      (bind _dialoguestate_49 (`self.AddDialogue` "Shrumer" "If you pass through that opening over there, your journey will begin!" (`|MakeArray`)))
      (switch `/Game/Blueprints/Dialogue/Enum_DialogueState` _dialoguestate_49
        (:`NewEnumerator0`
          (`self.ClearDialogueProgress`)
          (`self.CloseConversation`))))))