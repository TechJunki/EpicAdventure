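; Dialogue component for interacting with a cat, playing the player's spoken reactions to it.
; It overrides the parent Dialogue function and switches on the active dialogue branch: a default warning-off line, or a squirt-gun hint for the Portal Spawned branch.
; Each branch shows a single line with a continue option, then clears dialogue progress and closes the conversation.
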(fn `Dialogue`
  (`parent.Dialogue`)
  (switch `name` (`self.ActiveDialogueBranch`)
    (:`Default`
      (bind _dialoguestate (`self.AddDialogue` "Me" "Yikes! That cat looks mean enough to eat my lunch and my lunchbox. Good thing I don’t need to go back there!" (`|MakeArray` (make `/Game/Blueprints/Dialogue/Struct_Options` ">") :!type "/Game/Blueprints/Dialogue/Struct_Options Structure")))
      (switch `/Game/Blueprints/Dialogue/Enum_DialogueState` _dialoguestate
        (:`NewEnumerator0`
          (`self.ClearDialogueProgress`)
          (`self.CloseConversation`))))
    (:`PortalSpawned`
      (bind _dialoguestate_2 (`self.AddDialogue` "Me" "Great, now I have to deal with Captain Grumpy Whiskers. Maybe a squirt gun will make him rethink his life choices!" (`|MakeArray` (make `/Game/Blueprints/Dialogue/Struct_Options` ">") :!type "/Game/Blueprints/Dialogue/Struct_Options Structure")))
      (switch `/Game/Blueprints/Dialogue/Enum_DialogueState` _dialoguestate_2
        (:`NewEnumerator0`
          (`self.ClearDialogueProgress`)
          (`self.CloseConversation`))))))