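; BP_Cat is a start-level cat NPC that the player can talk to through its ACCatInteraction component.
; Entering its capsule turns it toward the player, plays a hiss and looping attack animation, locks input to UI and starts auto dialogue; leaving restores idle and resets the DoOnce.
; Actor overlap toggles an outline and, if tagged, a floating symbol via ACOutlinerAdvanced.
; PortalSpawned switches the dialogue branch and sets an exclamation-mark symbol.
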(event `PortalSpawned`
  (set `/Game/Blueprints/Dialogue/AC_Dialogue_Base.ActiveDialogueBranch` "PortalSpawned" (`self.AC_CatInteraction`))
  (set `self.Symbol Mesh` "/Game/Hyper/ResourcePack/Props/Symbols/Mesh/SM_Symbol_ExclamationMark.SM_Symbol_ExclamationMark"))

(event `self.CapsuleComponent.OnComponentBeginOverlap`
  (params (OverlappedComponent :type "PrimitiveComponent Object Reference") (OtherActor :type "Actor Object Reference") (OtherComp :type "PrimitiveComponent Object Reference") (OtherBodyIndex :type Integer) (bFromSweep :type Boolean) (SweepResult :type "HitResult Structure (by ref)"))
  (bind _returnvalue (`GameplayStatics.GetPlayerCharacter` 0))
  (bind _mesh (`self.Mesh`))
  (if (== OtherActor _returnvalue)
    (`/Engine/EditorBlueprintResources/StandardMacros.DoOnce` false :!label _label
      (:`Completed`
        (`self.K2_SetActorRotation` (`KismetMathLibrary.MakeRotFromX` (- (`self.K2_GetActorLocation` _returnvalue) (`self.K2_GetActorLocation` self))))
        (`GameplayStatics.PlaySoundAtLocation` "/Game/SFX/CatHissing.CatHissing" (`SceneComponent.K2_GetComponentLocation` _mesh) (struct) 1.0 1.0 0.0 null null null null)
        (`SkeletalMeshComponent.PlayAnimation` _mesh "/Game/StylizedCreaturesBundle/Animations/Cat/A_Cat_Combat_Unarmed_Attack01.A_Cat_Combat_Unarmed_Attack01" true)
        (`WidgetBlueprintLibrary.SetInputMode_UIOnlyEx` (`GameplayStatics.GetPlayerController` 0) null "DoNotLock" true)
        (message `/Game/Blueprints/Dialogue/BPI_Interactable.OverlapAutoDialogue` OtherActor)
        (`KismetSystemLibrary.PrintString` "OverlapAutoDialogue Called")))))

(event `/Game/Blueprints/Dialogue/BPI_Interactable.Interact`
  (params (Instigator :type "Actor Object Reference"))
  (set `self.InteractInstigator` Instigator)
  (`/Game/Blueprints/Dialogue/AC_Dialogue_Base.OpenConversation` (`self.AC_CatInteraction`)))

(event `self.ReceiveBeginPlay`)

(event `self.CapsuleComponent.OnComponentEndOverlap`
  (params (OverlappedComponent :type "PrimitiveComponent Object Reference") (OtherActor :type "Actor Object Reference") (OtherComp :type "PrimitiveComponent Object Reference") (OtherBodyIndex :type Integer))
  (if (== (`GameplayStatics.GetPlayerCharacter` 0) OtherActor)
    (if (not (`PrimitiveComponent.IsOverlappingActor` OverlappedComponent OtherActor))
      (`|ExecutionSequence`
        (:`then_0`
          (goto _label :!via `Reset`))
        (:`then_1`
          (`SkeletalMeshComponent.PlayAnimation` (`self.Mesh`) "/Game/StylizedCreaturesBundle/Animations/Cat/A_Cat_Idle01.A_Cat_Idle01" true))))))

(event `self.ReceiveActorBeginOverlap`
  (params (OtherActor :type "Actor Object Reference"))
  (if (== OtherActor (`GameplayStatics.GetPlayerCharacter` 0))
    (set `self.Overlapped?` true)
    (`/Game/Hyper/Outliner_System/Blueprints/AC_Outliner_Abstract.Switch Outline On Actor` (`self.AC_Outliner_Advanced`) self "NewEnumerator1" (`self.Overlapped?`) "NewEnumerator2")
    (if (`self.ActorHasTag` self "symbol")
      (`/Game/Hyper/Outliner_System/Blueprints/AC_Outliner_Abstract.Server: Spawn Replicated Symbol` (`self.AC_Outliner_Advanced`) (`KismetMathLibrary.MakeTransform` (0.0 0.0 150.0) (struct) (3.0 3.0 3.0)) true 15.0 1.0 true 1.0 (`self.Symbol Mesh`) "symbol" true self)
      (`KismetSystemLibrary.PrintString` "SPAWNEDDDD"))))

(event `self.ReceiveActorEndOverlap`
  (params (OtherActor :type "Actor Object Reference"))
  (bind _ac_outliner_advanced (`self.AC_Outliner_Advanced`))
  (bind (_symbol_attached _symbol_actor_attached) (`/Game/Hyper/Outliner_System/Blueprints/AC_Outliner_Abstract.Check if actor has symbol attached` _ac_outliner_advanced self))
  (if (== (`GameplayStatics.GetPlayerCharacter` 0) OtherActor)
    (set `self.Overlapped?` false)
    (`/Game/Hyper/Outliner_System/Blueprints/AC_Outliner_Abstract.Switch Outline On Actor` (`self.AC_Outliner_Advanced`) self "NewEnumerator1" (`self.Overlapped?`) "NewEnumerator2")
    (if _symbol_attached
      (`/Game/Hyper/Outliner_System/Blueprints/AC_Outliner_Abstract.Destroy symbol by actror` _ac_outliner_advanced _symbol_actor_attached))))

(fn `UserConstructionScript`
  (`parent.UserConstructionScript`))