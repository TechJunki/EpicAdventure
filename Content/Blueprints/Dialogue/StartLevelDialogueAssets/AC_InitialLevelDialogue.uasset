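; Dialogue component for the initial level: Mom sends the player outside before lunch, then the player declares they will gear up for adventure.
; Overrides the parent Dialogue function with two AddDialogue steps, each with voice audio and a single reply option.
; Each step advances on the Pass Through state; the first blends the camera to the player character before the monologue.
; The second clears dialogue progress and closes the conversation.
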(fn `Dialogue`
  (`parent.Dialogue`)
  (bind _dialoguestate (`self.AddDialogue` "Mom" "Go outside and play for a bit, sweetie. Lunch will be ready soon!" (`|MakeArray` (make `/Game/Blueprints/Dialogue/Struct_Options` "Okay mom!" "/Game/Blueprints/Dialogue/VOAudio/CharacterAudio/Okay_mom.Okay_mom") :!type "/Game/Blueprints/Dialogue/Struct_Options Structure") "/Game/Blueprints/Dialogue/VOAudio/MomAudio/Go_outside_and_play_for_a_bit_sweetie_Lunch_will_be_ready_soon.Go_outside_and_play_for_a_bit_sweetie_Lunch_will_be_ready_soon"))
  (switch `/Game/Blueprints/Dialogue/Enum_DialogueState` _dialoguestate
    (:`NewEnumerator0`
      (`PlayerController.SetViewTargetWithBlend` (`GameplayStatics.GetPlayerController` 0) (`GameplayStatics.GetPlayerCharacter` 0) 1.0 "VTBlend_Linear" 0.0 false)
      (bind _dialoguestate_2 (`self.AddDialogue` "Me" "Outside again, huh? Well, heroes don’t sit around waiting for lunch! If I’m gonna save the day, I’ll need my sword, my shield, and my trusty squirt gun. Time to gear up and get ready for adventure!" (`|MakeArray` (make `/Game/Blueprints/Dialogue/Struct_Options` "Let's do this!" "/Game/Blueprints/Dialogue/VOAudio/CharacterAudio/Lets_do_this.Lets_do_this") :!type "/Game/Blueprints/Dialogue/Struct_Options Structure") "/Game/Blueprints/Dialogue/VOAudio/CharacterAudio/Outside_again_huh_Well_heroes_dont_sit_around_waiting_for_lunch.Outside_again_huh_Well_heroes_dont_sit_around_waiting_for_lunch"))
      (switch `/Game/Blueprints/Dialogue/Enum_DialogueState` _dialoguestate_2
        (:`NewEnumerator0`
          (`self.ClearDialogueProgress`)
          (`self.CloseConversation`))))))