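; Dialogue component for a trash can whose lid the player wants as a shield, voicing the player character's comments on it.
; Its Dialogue override scans the Game Instance's inventory item messages for the sword and switches the active branch when found.
; Each branch plays one voiced line, either hinting to find the sword or to knock the lid loose, then clears progress and closes the conversation.
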(event `self.ReceiveBeginPlay`
  (`parent.ReceiveBeginPlay`))

(fn `Dialogue`
  (`parent.Dialogue`)
  (bind _inventoryitems (message `/Game/Blueprints/BPIs/BPI_InGameUpdates.GetInventoryItems` (`GameplayStatics.GetGameInstance`)))
  (for _array_element _inventoryitems
    (if (`KismetStringLibrary.EqualEqual_StrStr` _array_element "Sword1")
      (set `self.ActiveDialogueBranch` "HasSword")
      (break)))
  (switch `name` (`self.ActiveDialogueBranch`)
    (:`Default`
      (bind _dialoguestate (`self.AddDialogue` "Me" "That lid would make a great shield… if I could just knock it loose. Guess I’ll need my sword for that. Now, where did I leave it?" (`|MakeArray`) "/Game/Blueprints/Dialogue/VOAudio/CharacterAudio/That_lid_would_make_a_great_shield.That_lid_would_make_a_great_shield"))
      (switch `/Game/Blueprints/Dialogue/Enum_DialogueState` _dialoguestate
        (:`NewEnumerator0`
          (`self.ClearDialogueProgress`)
          (`self.CloseConversation`))))
    (:`HasSword`
      (bind _dialoguestate_2 (`self.AddDialogue` "Me" "Got the sword—now let’s give this trashcan a little ‘heroic adjustment.’" (`|MakeArray`) "/Game/Blueprints/Dialogue/VOAudio/CharacterAudio/Got_the_sword_now_lets.Got_the_sword_now_lets"))
      (switch `/Game/Blueprints/Dialogue/Enum_DialogueState` _dialoguestate_2
        (:`NewEnumerator0`
          (`self.ClearDialogueProgress`)
          (`self.CloseConversation`))))))