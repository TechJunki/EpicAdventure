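; BP_PortalDialogue is a trigger actor that starts an automatic portal dialogue when the player walks into its capsule.
; The first player overlap switches to UI-only input and, after a short delay, sends the OverlapAutoDialogue message to the player character.
; Its Interact event waits, blends the camera to the player, then opens the ACPortalSpawned conversation once.
; Its own OverlapAutoDialogue event destroys the actor after a brief delay.
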(event `self.CapsuleComponent.OnComponentBeginOverlap`
  (params (OverlappedComponent :type "PrimitiveComponent Object Reference") (OtherActor :type "Actor Object Reference") (OtherComp :type "PrimitiveComponent Object Reference") (OtherBodyIndex :type Integer) (bFromSweep :type Boolean) (SweepResult :type "HitResult Structure (by ref)"))
  (bind _returnvalue (`GameplayStatics.GetPlayerCharacter` 0))
  (if (== OtherActor _returnvalue)
    (`/Engine/EditorBlueprintResources/StandardMacros.DoOnce` false
      (:`Completed`
        (`WidgetBlueprintLibrary.SetInputMode_UIOnlyEx` (`GameplayStatics.GetPlayerController` 0) null "DoNotLock" true)
        (`KismetSystemLibrary.Delay` 0.2)
        (message `/Game/Blueprints/Dialogue/BPI_Interactable.OverlapAutoDialogue` _returnvalue)
        (`KismetSystemLibrary.PrintString` "OverlapAutoDialogue Called")))))

(event `/Game/Blueprints/Dialogue/BPI_Interactable.Interact`
  (params (Instigator :type "Actor Object Reference"))
  (set `self.InteractInstigator` Instigator)
  (`KismetSystemLibrary.Delay` 2.0)
  (`PlayerController.SetViewTargetWithBlend` (`GameplayStatics.GetPlayerController` 0) (`GameplayStatics.GetPlayerCharacter` 0) 0.5 "VTBlend_Linear" 0.0 false)
  (`/Engine/EditorBlueprintResources/StandardMacros.DoOnce` false
    (:`Completed`
      (`/Game/Blueprints/Dialogue/AC_Dialogue_Base.OpenConversation` (`self.AC_PortalSpawned`)))))

(event `/Game/Blueprints/Dialogue/BPI_Interactable.OverlapAutoDialogue`
  (`KismetSystemLibrary.Delay` 0.2)
  (`self.K2_DestroyActor`))

(fn `UserConstructionScript`
  (`parent.UserConstructionScript`))