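; Dialogue component for the conversation with Mom about the player's missing toy sword, with voiced lines and player reply options.
; The Dialogue override first scans the GameInstance's inventory items and switches to the HasSword branch if Sword1 is present.
; The default branch points the player to the backyard tree, then sets MomSwordConvo2 as the follow-up branch.
; The follow-up and HasSword branches clear dialogue progress before closing.
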(fn `Dialogue`
  (`parent.Dialogue`)
  (bind _inventoryitems (message `/Game/Blueprints/BPIs/BPI_InGameUpdates.GetInventoryItems` (`GameplayStatics.GetGameInstance`)))
  (for _array_element _inventoryitems
    (if (`KismetStringLibrary.EqualEqual_StrStr` _array_element "Sword1")
      (set `self.ActiveDialogueBranch` "HasSword")
      (break)))
  (switch `name` (`self.ActiveDialogueBranch`)
    (:`Default`
      (bind _dialoguestate (`self.AddDialogue` "Me" "I really want to play a game, but I need my toy sword first. I think Mom might know where it is." (`|MakeArray` (make `/Game/Blueprints/Dialogue/Struct_Options` "I'll yell and ask mom!" "/Game/Blueprints/Dialogue/VOAudio/YellAndAskMom.YellAndAskMom") :!type "/Game/Blueprints/Dialogue/Struct_Options Structure") "/Game/Blueprints/Dialogue/VOAudio/IntroTTS-playgame.IntroTTS-playgame"))
      (switch `/Game/Blueprints/Dialogue/Enum_DialogueState` _dialoguestate
        (:`NewEnumerator0`
          (bind _dialoguestate_2 (`self.AddDialogue` "Me" "Hey Mom! ! !" (`|MakeArray`) "/Game/Blueprints/Dialogue/VOAudio/HeyMom.HeyMom"))
          (switch `/Game/Blueprints/Dialogue/Enum_DialogueState` _dialoguestate_2
            (:`NewEnumerator0`
              (bind (_dialoguestate_3 _optionindex) (`self.AddDialogue` "Mom" "Hey kiddo! What are you up to?" (`|MakeArray` (make `/Game/Blueprints/Dialogue/Struct_Options` " I want to play a game, but I can't find my toy sword. Do you know where it is?" "/Game/Blueprints/Dialogue/VOAudio/DoYouKnowwheresword.DoYouKnowwheresword") (make `/Game/Blueprints/Dialogue/Struct_Options` "I'm bored, Mom. Do you have any ideas for something fun to do?" "/Game/Blueprints/Dialogue/VOAudio/IdeasForFun.IdeasForFun") (make `/Game/Blueprints/Dialogue/Struct_Options` "Just hanging out. What are you doing, Mom?" "/Game/Blueprints/Dialogue/VOAudio/JustHanginout.JustHanginout") :!type "/Game/Blueprints/Dialogue/Struct_Options Structure") "/Game/Blueprints/Dialogue/VOAudio/Hey_kiddo_What_are_you_u_1.Hey_kiddo_What_are_you_u_1"))
              (switch `/Game/Blueprints/Dialogue/Enum_DialogueState` _dialoguestate_3
                (:`NewEnumerator0`
                  (switch `int` _optionindex
                    (:`0`
                      (bind _dialoguestate_4 (`self.AddDialogue` "Mom" "Hmm... Last time I saw it, it was near the tree in the backyard. Why don't you check there!?" (`|MakeArray`) "/Game/Blueprints/Dialogue/VOAudio/Hmm_Last_time_I_saw_it.Hmm_Last_time_I_saw_it"))
                      (switch `/Game/Blueprints/Dialogue/Enum_DialogueState` _dialoguestate_4
                        (:`NewEnumerator0`
                          (bind _dialoguestate_5 (`self.AddDialogue` "Me" "Thanks Mom! I'll go check by the tree! :)" (`|MakeArray`) "/Game/Blueprints/Dialogue/VOAudio/ThanksMomIllCheckbyTree.ThanksMomIllCheckbyTree"))
                          (switch `/Game/Blueprints/Dialogue/Enum_DialogueState` _dialoguestate_5
                            (:`NewEnumerator0`
                              (bind _dialoguestate_6 (`self.AddDialogue` "Me" "I'll try to find my Sword, my Shield, and my gun! Then I'll definitely be able to have some fun!" (`|MakeArray`) "/Game/Blueprints/Dialogue/VOAudio/TryToFindAll3.TryToFindAll3"))
                              (switch `/Game/Blueprints/Dialogue/Enum_DialogueState` _dialoguestate_6
                                (:`NewEnumerator0`
                                  (`self.SetDialogueBranch` "MomSwordConvo2")
                                  (`self.CloseConversation`))))))))
                    (:`1`
                      (bind _dialoguestate_7 (`self.AddDialogue` "Mom" "Well, you could always help me with some chores, but I bet you'd rather play with your toys. Have you found your toy sword yet?" (`|MakeArray`) "/Game/Blueprints/Dialogue/VOAudio/Well_you_could_always_he_1.Well_you_could_always_he_1"))
                      (switch `/Game/Blueprints/Dialogue/Enum_DialogueState` _dialoguestate_7
                        (:`NewEnumerator0`
                          (bind _dialoguestate_8 (`self.AddDialogue` "Mom" "Last time I saw it, it was in the backyard near the tree. Why don't you check there!?" (`|MakeArray`) "/Game/Blueprints/Dialogue/VOAudio/Last_time_I_saw_it_it_wa_1.Last_time_I_saw_it_it_wa_1"))
                          (switch `/Game/Blueprints/Dialogue/Enum_DialogueState` _dialoguestate_8
                            (:`NewEnumerator0`
                              (bind _dialoguestate_9 (`self.AddDialogue` "Me" "I'll try to find my Sword, my Shield, and my gun! Then I'll definitely be able to have some fun!" (`|MakeArray`) "/Game/Blueprints/Dialogue/VOAudio/TryToFindAll3.TryToFindAll3"))
                              (switch `/Game/Blueprints/Dialogue/Enum_DialogueState` _dialoguestate_9
                                (:`NewEnumerator0`
                                  (`self.SetDialogueBranch` "MomSwordConvo2")
                                  (`self.CloseConversation`))))))))
                    (:`2`
                      (bind _dialoguestate_10 (`self.AddDialogue` "Mom" "Just finishing up some work. Can you go pickup your sword that is outside? I think I saw it near the tree in the backyard." (`|MakeArray`) "/Game/Blueprints/Dialogue/VOAudio/Just_finishing_up_some_wo_1.Just_finishing_up_some_wo_1"))
                      (switch `/Game/Blueprints/Dialogue/Enum_DialogueState` _dialoguestate_10
                        (:`NewEnumerator0`
                          (bind _dialoguestate_11 (`self.AddDialogue` "Me" "I'll try to find my Sword, my Shield, and my gun! Then I'll definitely be able to have some fun!" (`|MakeArray`) "/Game/Blueprints/Dialogue/VOAudio/TryToFindAll3.TryToFindAll3"))
                          (switch `/Game/Blueprints/Dialogue/Enum_DialogueState` _dialoguestate_11
                            (:`NewEnumerator0`
                              (`self.SetDialogueBranch` "MomSwordConvo2")
                              (`self.CloseConversation`))))))))))))))
    (:`HasSword`
      (bind _dialoguestate_12 (`self.AddDialogue` "Mom" "I see you found your sword! Hope you have fun playing hero! I'll call you in when lunch is ready." (`|MakeArray` (struct) :!type "/Game/Blueprints/Dialogue/Struct_Options Structure") "/Game/Blueprints/Dialogue/VOAudio/I_see_you_found_your_swor_2.I_see_you_found_your_swor_2"))
      (switch `/Game/Blueprints/Dialogue/Enum_DialogueState` _dialoguestate_12
        (:`NewEnumerator0`
          (`self.ClearDialogueProgress`)
          (`self.CloseConversation`))))
    (:`MomSwordConvo2`
      (bind _dialoguestate_13 (`self.AddDialogue` "Me" "Mom! I can't find it!" (`|MakeArray`) "/Game/Blueprints/Dialogue/VOAudio/MomICantFindIt.MomICantFindIt"))
      (switch `/Game/Blueprints/Dialogue/Enum_DialogueState` _dialoguestate_13
        (:`NewEnumerator0`
          (bind (_dialoguestate_14 _optionindex_2) (`self.AddDialogue` "Mom" "Did you check by the tree in the backyard?" (`|MakeArray` (make `/Game/Blueprints/Dialogue/Struct_Options` "Yes") (make `/Game/Blueprints/Dialogue/Struct_Options` "No") :!type "/Game/Blueprints/Dialogue/Struct_Options Structure") "/Game/Blueprints/Dialogue/VOAudio/Did_you_check_by_the_tree_1.Did_you_check_by_the_tree_1"))
          (switch `/Game/Blueprints/Dialogue/Enum_DialogueState` _dialoguestate_14
            (:`NewEnumerator0`
              (switch `int` _optionindex_2
                (:`0`
                  (bind _dialoguestate_15 (`self.AddDialogue` "Mom" "You should go check again, and make sure to look all around the tree. I am pretty sure that's where you left it!" (`|MakeArray` (make `/Game/Blueprints/Dialogue/Struct_Options` "Okay!") :!type "/Game/Blueprints/Dialogue/Struct_Options Structure") "/Game/Blueprints/Dialogue/VOAudio/You_should_go_check_again_2.You_should_go_check_again_2"))
                  (switch `/Game/Blueprints/Dialogue/Enum_DialogueState` _dialoguestate_15
                    (:`NewEnumerator0`
                      (`self.ClearDialogueProgress`)
                      (`self.CloseConversation`))))
                (:`1`
                  (bind _dialoguestate_16 (`self.AddDialogue` "Mom" "Make sure to look all around the tree in the back. I am pretty sure that's where you left it!" (`|MakeArray` (make `/Game/Blueprints/Dialogue/Struct_Options` "Okay!") :!type "/Game/Blueprints/Dialogue/Struct_Options Structure") "/Game/Blueprints/Dialogue/VOAudio/Make_sure_to_look_all_aro_1.Make_sure_to_look_all_aro_1"))
                  (switch `/Game/Blueprints/Dialogue/Enum_DialogueState` _dialoguestate_16
                    (:`NewEnumerator0`
                      (`self.ClearDialogueProgress`)
                      (`self.CloseConversation`))))))))))))