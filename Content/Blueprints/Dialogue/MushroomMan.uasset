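; Mushroom Man dialogue NPC that starts a conversation when interacted with.
; Interact stores the instigator and opens the conversation through the ACMushroomMan component.
; When the conversation closes, it restores game-only input for the first player controller, hides the mouse cursor and loops the idle animation on the mesh.
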(event `/Game/Blueprints/Dialogue/BPI_Interactable.Interact`
  (params (Instigator :type "Actor Object Reference"))
  (set `self.InteractInstigator` Instigator)
  (`/Game/Blueprints/Dialogue/AC_Dialogue_Base.OpenConversation` (`self.AC_MushroomMan`)))

(event `/Game/Blueprints/Dialogue/BPI_Interactable.ConversationClosed`
  (bind _returnvalue (`GameplayStatics.GetPlayerController` 0))
  (`WidgetBlueprintLibrary.SetInputMode_GameOnly` _returnvalue)
  (set `PlayerController.bShowMouseCursor` false _returnvalue)
  (`SkeletalMeshComponent.PlayAnimation` (`self.Mesh`) "/Game/Characters/MushroomMan/MushroomIdleMontage.MushroomIdleMontage" true))

(fn `UserConstructionScript`
  (`parent.UserConstructionScript`))