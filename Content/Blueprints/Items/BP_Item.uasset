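; BP_Item is a pickup item that highlights itself while the player character overlaps it.
; Overlap toggles an outline through ACOutlinerAdvanced and, for actors tagged "symbol", spawns a replicated down-arrow above the item.
; PickupItem returns the Item value and calls DestroyItem, which clears outline and symbol, then destroys the actor after a short delay.
; Ending overlap reuses that cleanup branch without destroying the item.
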(event `CustomEvent`
  (`self.PickupItem`))

(event `DestroyItem`
  (bind _ac_outliner_advanced (`self.AC_Outliner_Advanced`))
  (bind (_symbol_attached _symbol_actor_attached) (`/Game/Hyper/Outliner_System/Blueprints/AC_Outliner_Abstract.Check if actor has symbol attached` _ac_outliner_advanced self))
  (`|ExecutionSequence`
    (:`then_0`
      (set `self.Overlapped?` false :!label _label)
      (`/Game/Hyper/Outliner_System/Blueprints/AC_Outliner_Abstract.Switch Outline On Actor` (`self.AC_Outliner_Advanced`) self "NewEnumerator1" (`self.Overlapped?`) "NewEnumerator2")
      (if _symbol_attached
        (`/Game/Hyper/Outliner_System/Blueprints/AC_Outliner_Abstract.Destroy symbol by actror` _ac_outliner_advanced _symbol_actor_attached)))
    (:`then_1`
      (`KismetSystemLibrary.Delay` 0.1)
      (`self.K2_DestroyActor`))))

(event `self.ReceiveActorBeginOverlap`
  (params (OtherActor :type "Actor Object Reference"))
  (if (== OtherActor (`GameplayStatics.GetPlayerCharacter` 0))
    (set `self.Overlapped?` true)
    (`/Game/Hyper/Outliner_System/Blueprints/AC_Outliner_Abstract.Switch Outline On Actor` (`self.AC_Outliner_Advanced`) self "NewEnumerator1" (`self.Overlapped?`) "NewEnumerator2")
    (if (`self.ActorHasTag` self "symbol")
      (`/Game/Hyper/Outliner_System/Blueprints/AC_Outliner_Abstract.Server: Spawn Replicated Symbol` (`self.AC_Outliner_Advanced`) (`KismetMathLibrary.MakeTransform` (0.0 0.0 150.0) (struct) (3.0 3.0 3.0)) true 15.0 1.0 true 1.0 "/Game/Hyper/ResourcePack/Props/Symbols/Mesh/SM_Symbol_Arrow_Down.SM_Symbol_Arrow_Down" "symbol" true self)
      (`KismetSystemLibrary.PrintString` "SPAWNEDDDD"))))

(event `self.ReceiveActorEndOverlap`
  (params (OtherActor :type "Actor Object Reference"))
  (if (== (`GameplayStatics.GetPlayerCharacter` 0) OtherActor)
    (goto _label)))

(fn `PickupItem`
  (returns (Item :type String))
  (`KismetSystemLibrary.PrintString` "Item Picked Up")
  (`self.DestroyItem`)
  (return (`self.Item`)))

(fn `UserConstructionScript`)