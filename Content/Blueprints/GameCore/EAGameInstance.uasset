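; EAGameInstance is a game instance that holds player data so it can persist across level loads.
; It stores the selected character class, hair, skin and clothes style indices, current and max health, inventory items, and the save slot name.
; Each piece of data has a simple setter event and a matching getter function, with no validation or save-to-disk logic.
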(event `/Game/Blueprints/BPIs/BPI_ChangeCharacterStyleInterface.SetSelectedCharacter`
  (params (SelectedCharacterClass :type "Pawn Class Reference"))
  (set `self.SelectedCharacter` SelectedCharacterClass))

(event `/Game/Blueprints/BPIs/BPI_ChangeCharacterStyleInterface.SetCharacterStyle`
  (params (HairInt :type Integer) (SkinInt :type Integer) (ClothesInt :type Integer))
  (set `self.SetHairInt` HairInt)
  (set `self.SetSkinInt` SkinInt)
  (set `self.SetClothesInt` ClothesInt))

(event `/Game/Blueprints/BPIs/BPI_SaveGameSlot.SaveGameSlotName`
  (params (SaveSlotName :type String))
  (set `self.SetSaveSlotName` SaveSlotName))

(event `/Game/Blueprints/BPIs/BPI_InGameUpdates.SetCharacterHealth`
  (params (CurrentHealth :type Integer) (MaxHealth :type Integer))
  (set `self.SetCurrentHealth` CurrentHealth)
  (set `self.SetMaxHealth` MaxHealth))

(event `/Game/Blueprints/BPIs/BPI_InGameUpdates.SetInventoryItems`
  (params (Inventory :type "Array of String (by ref)"))
  (set `self.SetInventory Items` Inventory))

(fn `GetCharacterHealth`
  (returns (CurrentHealth :type Integer) (MaxHealth :type Integer))
  (return (`self.SetCurrentHealth`) (`self.SetMaxHealth`)))

(fn `GetCharacterStyle`
  (returns (HairInt :type Integer) (SkinInt :type Integer) (ClothesInt :type Integer))
  (return (`self.SetHairInt`) (`self.SetSkinInt`) (`self.SetClothesInt`)))

(fn `GetGameSlotName`
  (returns (GameSaveSlotName :type String))
  (return (`self.SetSaveSlotName`)))

(fn `GetInventoryItems`
  (returns (InventoryItems :type "Array of String"))
  (return (`self.SetInventory Items`)))

(fn `GetSelectedCharacter`
  (returns (SelectedCharacterClass :type "Pawn Class Reference"))
  (return (`self.SelectedCharacter`)))