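; BP_Pillar is a placeable magic ice pillar that serves as both build preview and spawned pillar.
; EnableBuild and DisableBuild use paired DoOnce gates to toggle placeability, material and looping Cryonis animation.
; CheckForOverlap box-traces the space, ignoring one custom object type and treating the first other hit as blocking unless it simulates physics.
; When placeable, SpawnTower spawns another BP_Pillar, which enables collision, animates once and grows its collision box via timeline.
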(event `EnableBuild`
  (bind _pillar (`self.Pillar`))
  (bind _pillar_2 (`self.Pillar`))
  (`|ExecutionSequence`
    (:`then_0`
      (`/Engine/EditorBlueprintResources/StandardMacros.DoOnce` false :!label _label
        (:`Completed`
          (`SkeletalMeshComponent.PlayAnimation` _pillar_2 "/Game/Mechanics/MagicPillar/CryonisIce_Anim.CryonisIce_Anim" true)
          (set `self.CanPlace` true)
          (`PrimitiveComponent.SetMaterial` _pillar 0 "/Game/Mechanics/MagicPillar/MI_Enable.MI_Enable"))))
    (:`then_1`
      (goto _label_2 :!via `Reset`))))

(event `DisableBuild`
  (bind _pillar (`self.Pillar`))
  (`|ExecutionSequence`
    (:`then_0`
      (`/Engine/EditorBlueprintResources/StandardMacros.DoOnce` false :!label _label_2
        (:`Completed`
          (`SkeletalMeshComponent.Stop` _pillar)
          (`SkeletalMeshComponent.SetMorphTarget` _pillar "Short" 0.0 true)
          (set `self.CanPlace` false)
          (`PrimitiveComponent.SetMaterial` (`self.Pillar`) 0 "/Game/Mechanics/MagicPillar/MI_Disable.MI_Disable"))))
    (:`then_1`
      (goto _label :!via `Reset`))))

(event `ExpandCollision`
  (bind _collision (`self.Collision`))
  (bind (_boxextent_x _boxextent_y _boxextent_z) (`KismetMathLibrary.BreakVector` (`BoxComponent.BoxExtent` _collision)))
  (bind (_direction _alpha) (`Timeline|Timeline`)
    (:`Update`
      (bind _returnvalue (`KismetMathLibrary.Lerp` _boxextent_z 100.0 _alpha))
      (`BoxComponent.SetBoxExtent` _collision (`KismetMathLibrary.MakeVector` _boxextent_x _boxextent_y _returnvalue) true)
      (`SceneComponent.K2_SetRelativeLocation` _collision (`KismetMathLibrary.MakeVector` 0.0 0.0 _returnvalue) false false))))

(fn `CheckForOverlap`
  (returns (ReturnValue :type Boolean))
  (locals (OverlappingObjects :type Boolean :default false))
  (bind _box (`self.Box`))
  (bind _returnvalue (`SceneComponent.K2_GetComponentLocation` _box))
  (bind _outhits (`KismetSystemLibrary.BoxTraceMulti` _returnvalue _returnvalue (`BoxComponent.GetScaledBoxExtent` _box) (`SceneComponent.K2_GetComponentRotation` _box) "TraceTypeQuery1"))
  (for _array_element _outhits
    (bind (_bblockinghit _binitialoverlap _time _distance _location _impactpoint _normal _impactnormal _physmat _hitactor _hitcomponent) (`GameplayStatics.BreakHitResult` _array_element))
    (if (`|EnumInequality` (`PrimitiveComponent.GetCollisionObjectType` _hitcomponent) "ECC_GameTraceChannel1")
      (set `local.OverlappingObjects` (not (`SceneComponent.IsSimulatingPhysics` _hitcomponent "None")))
      (break)))
  (return (not (`local.OverlappingObjects`))))

(fn `OnSpawned`
  (`PrimitiveComponent.SetCollisionEnabled` (`self.Collision`) "QueryAndPhysics")
  (`PrimitiveComponent.SetCollisionEnabled` (`self.Pillar`) "QueryAndPhysics")
  (`SkeletalMeshComponent.PlayAnimation` (`self.Pillar`) "/Game/Mechanics/MagicPillar/CryonisIce_Anim.CryonisIce_Anim" false)
  (`self.ExpandCollision`))

(fn `SpawnTower`
  (params (Transform :type "Transform Structure"))
  (if (`self.CanPlace`)
    (bind _returnvalue (`|SpawnActorFromClass` "BP_Pillar_C" Transform "Undefined" "MultiplyWithRoot" null null))
    (`self.OnSpawned` _returnvalue)))

(fn `UserConstructionScript`)